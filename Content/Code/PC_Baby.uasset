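; Player controller that runs a UMG body-part assembly game, where parts move from a conveyor to a table and then decide a series of minigames.
; A picked-up part becomes a widget that follows the mouse on Tick, with drops committing it and right-click returning it to the conveyor.
; When all slots fill, the four limb variants plus a trailing NONE select minigame widgets, each GameOver advancing to the next.
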(event Custom|next%20please
  (bind _currentminigame (Variables|Default|GetCurrentMinigame))
  (|Shitstuff_2 (Utilities|Array|Get(acopy) (Variables|Default|GetVariants) (Variables|Default|GetminigameIndex)))
  (UserInterface|Viewport|AddtoViewport _currentminigame 0)
  (EventDispatchers|BindEventtoGameOver _currentminigame (delegate Custom|Minigame%20Done))
  (Variables|/Script/UMG.UserWidget|SetbIsFocusable _currentminigame true)
  (Variables|/Script/UMG.UserWidget|SetbIsFocusable (Variables|Default|GetMain) false))

(event Custom|Slots%20full%20w/e
  (params (LeftArm :type E_PartVariant%20Enum :default "NewEnumerator0") (RightArm :type E_PartVariant%20Enum :default "NewEnumerator0") (LeftLeg :type E_PartVariant%20Enum :default "NewEnumerator0") (RightLeg :type E_PartVariant%20Enum :default "NewEnumerator0"))
  (bind _currentminigame (Variables|Default|GetCurrentMinigame))
  (|Initminigamevariants_2 LeftArm RightArm LeftLeg RightLeg)
  (|Shitstuff_2 (Utilities|Array|Get(acopy) (Variables|Default|GetVariants) (Variables|Default|GetminigameIndex)))
  (UserInterface|Viewport|AddtoViewport _currentminigame 0)
  (EventDispatchers|BindEventtoGameOver _currentminigame (delegate Custom|Minigame%20Done))
  (Variables|/Script/UMG.UserWidget|SetbIsFocusable _currentminigame true)
  (Variables|/Script/UMG.UserWidget|SetbIsFocusable (Variables|Default|GetMain) false))

(event Custom|Minigame%20Done
  (bind _currentminigame (Variables|Default|GetCurrentMinigame))
  (bind _result (Math|Integer|IncrementInt (Variables|Default|GetminigameIndex))
    (:%20%20
      (EventDispatchers|UnbindEventfromGameOver _currentminigame (delegate Custom|Minigame%20Done))
      (Widget|RemovefromParent _currentminigame)
      (if (> _result 4)
        (Variables|/Script/UMG.UserWidget|SetbIsFocusable (Variables|Default|GetMain) true)
        (else
          (CallFunction|NextPlease))))))

(event EventBeginPlay
  (bind _returnvalue (Game|GetPlayerController 0))
  (bind _returnvalue_2 (UserInterface|CreateWidget "/Game/Code/Widgets/W_Main.W_Main_C" _returnvalue))
  (Variables|Default|SetMain _returnvalue_2)
  (Variables|Default|SetTable (Variables|/Game/Code/Widgets/W_Main.W_Main_C|GetW_Table _returnvalue_2))
  (Variables|Default|SetConveyor (Variables|/Game/Code/Widgets/W_Main.W_Main_C|GetW_Conveyor _returnvalue_2))
  (UserInterface|Viewport|AddtoViewport _returnvalue_2 0)
  (Input|SetInputModeGameandUI _returnvalue _returnvalue_2 "DoNotLock" false)
  (EventDispatchers|BindEventtoBodyPartTaken (Variables|Default|GetConveyor) (EventDispatchers|CreateEvent :!event ItemPickedUp))
  (EventDispatchers|BindEventtoAllSlotsFilled (Variables|Default|GetTable) (delegate Custom|Slots%20full%20w/e)))

(event EventTick
  (params (DeltaSeconds :type Float%20%28single-precision%29))
  (bind _helditem (Variables|Default|GetheldItem))
  (Utilities|IsValid (Variables|Default|GetheldItem)
    (:Is%20Valid
      (bind _returnvalue (Class|WidgetLayoutLibrary|GetMousePositiononViewport))
      (Class|UserWidget|SetPositioninViewport _helditem (- _returnvalue (/ (Class|Widget|GetDesiredSize (Variables|/Game/Code/Widgets/W_BodyPart.W_BodyPart_C|GetAnImage _helditem)) 2.0)) false))))

(event Input|MouseEvents|RightMouseButton
  (params (Key :type Key%20Structure :default "None"))
  (:Pressed
    (Utilities|IsValid (Variables|Default|GetheldItem)
      (:Is%20Valid
        (Default|ItemReturned (Variables|Default|GetConveyor))
        (Widget|RemovefromParent (Variables|Default|GetheldItem))
        (Variables|Default|SetheldItem 0)))))

(event Input|MouseEvents|LeftMouseButton
  (params (Key :type Key%20Structure :default "None"))
  (:Pressed
    (Variables|Default|SetLMBIsDown true)
    (Default|CallLMBPressed))
  (:Released
    (Variables|Default|SetLMBIsDown false)
    (Default|CallLMBReleased)))

(fn ConstructionScript)

(fn ItemPickedUp
  (params (Taken%20Part :type W%20Body%20Part%20Object%20Reference))
  (bind _returnvalue (UserInterface|CreateWidget "/Game/Code/Widgets/W_BodyPart.W_BodyPart_C" (Game|GetPlayerController 0)))
  (Default|FromBodyPart _returnvalue Taken%20Part)
  (bind _output_get (Variables|Default|SetheldItem _returnvalue))
  (EventDispatchers|BindEventtoDropped _output_get (EventDispatchers|CreateEvent :!event HeldItemDropped))
  (UserInterface|Viewport|AddtoViewport _output_get 0)
  (Variables|/Game/Code/Widgets/Table/W_Table.W_Table_C|SetPickedUpPart (Variables|Default|GetTable) (Variables|Default|GetheldItem)))

(fn HeldItemDropped
  (params (Me :type W%20Body%20Part%20Object%20Reference))
  (Widget|RemovefromParent Me)
  (Variables|Default|SetheldItem 0)
  (Default|ItemCommited (Variables|Default|GetConveyor)))